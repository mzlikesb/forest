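; BP_NPC is a conversational NPC that replies to the player with AI-generated speech and lip sync.
; User messages from BP_Character go through APIClient to ChatGPT; the reply is broadcast, then sent to TTS.
; Returned audio is processed at runtime by OVRLipSync's offline model, driving viseme morph targets during playback.
; Tick eases a look target toward a nearby player's camera or a default point, while a self-recalling event randomizes blinks.
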(event `self.OVRLipSyncPlaybackActor.OnVisemesReady`
  (`OVRLipSyncActorComponentBase.AssignVisemesToMorphTargets` :`self` (`self.OVRLipSyncPlaybackActor`)))

(event `self.ReceiveBeginPlay`
  (`|ExecutionSequence`
    (:`then_0`
      (`self.Blink`))
    (:`then_1`
      (bind _returnvalue (`GameplayStatics.GetActorOfClass` "/Game/Frameworks/BP_Character.BP_Character_C"))
      (bind _output_get (set `self.Player` _returnvalue))
      (add `/Game/Frameworks/BP_Character.OnReceiveMessage` _output_get (delegate `OnReceiveUserMessage`)))))

(event `OnReceiveUserMessage`
  (params (Text :type String) (bIsUser :type Boolean))
  ;[1 1 1] Callbacks
  (if bIsUser
    (`APIClient.SendChatGPTRequest` (`self.APIClient`) (`self.System Prompt`) Text)))

(event `self.APIClient.OnChatGPTResponse`
  (params (Text :type String))
  ;[1 1 1] Callbacks
  (`self.OnReceiveMessage` Text)
  (`APIClient.SendTTSRequest` (`self.APIClient`) Text))

(event `self.APIClient.OnTTSResponse`
  (params (Data :type "Array of Byte"))
  (bind _ovrlipsyncplaybackactor (`self.OVRLipSyncPlaybackActor`))
  ;[1 1 1] Callbacks
  (bind _returnvalue (`APIClient.LoadSoundWave` (`self.APIClient`) Data))
  (bind _returnvalue_2 (`OVRLipSyncPlaybackActorComponent.OVRLipSyncProcessSoundWave` (`self.OVRLipSyncPlaybackActor`) Data true))
  (if _returnvalue_2
    (`AudioComponent.SetSound` (`self.Audio`) _returnvalue)
    (`/Engine/EditorBlueprintResources/StandardMacros.IsValid` (`OVRLipSyncPlaybackActorComponent.ProcessedSequence` _ovrlipsyncplaybackactor)
      (:`Is Valid`
        (`OVRLipSyncPlaybackActorComponent.Start` _ovrlipsyncplaybackactor (`self.Audio`) (`OVRLipSyncPlaybackActorComponent.ProcessedSequence` _ovrlipsyncplaybackactor))))))

(event `self.ReceiveTick`
  (params (DeltaSeconds :type "Float (single-precision)"))
  (bind _target (`self.FindTarget`))
  (bind _targetlocation (`self.LookTarget` _target))
  (bind _output_get (set `self.PrevTarget` (`self.Target`)))
  (set `self.Target` (`KismetMathLibrary.VLerp` _output_get _targetlocation (* DeltaSeconds 5.0))))

(event `Blink`
  ;[1 1 1] Blink
  (`KismetSystemLibrary.Delay` (`KismetMathLibrary.RandomFloatInRange` 2.0 10.0))
  (`TimelineComponent.PlayFromStart` (`self.BlinkTimeline`))
  (`KismetSystemLibrary.Delay` 0.5)
  (`self.Blink`))

(fn `FindTarget`
  (returns (Target :type "Actor Object Reference"))
  (bind (_outactors _returnvalue) (`KismetSystemLibrary.SphereOverlapActors` (`self.K2_GetActorLocation`) (`self.Interaction Range`) (`|MakeArray` "ObjectTypeQuery3" :!type "EObjectTypeQuery Enum") "/Game/Frameworks/BP_Character.BP_Character_C"))
  (if _returnvalue
    (return (`|GetArrayItem` _outactors))
    (else
      (return null))))

(fn `LookTarget`
  (params (Target :type "Actor Object Reference"))
  (returns (TargetLocation :type "Vector Structure"))
  (bind _capsule (`self.Capsule`))
  (`/Engine/EditorBlueprintResources/StandardMacros.IsValid` Target
    (:`Is Valid`
      (bind _asbp_character (cast `/Game/Frameworks/BP_Character` Target)
        (:`then`
          (bind _camera (`/Game/Frameworks/BP_Character.Camera` _asbp_character))
          (`/Engine/EditorBlueprintResources/StandardMacros.IsValid` _camera
            (:`Is Valid`
              (return (`SceneComponent.K2_GetComponentLocation` _camera)))
            (:`Is Not Valid`
              _)))
        (:`CastFailed`
          _)))
    (:`Is Not Valid`
      _))
  (return (+ (`SceneComponent.K2_GetComponentLocation` _capsule) (0.0 0.0 160.0) (* (`SceneComponent.GetRightVector` _capsule) (`self.Interaction Range`)))))

(fn `UserConstructionScript`
  (bind _targetlocation (`self.LookTarget` null))
  (set `self.Target` _targetlocation))