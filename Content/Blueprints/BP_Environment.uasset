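; Environment actor that configures a FireFlies particle effect when play begins, setting its color and wind speed scale parameters.
; It also holds an unconnected Timeline graph that never runs.
; That graph would loop color blends for grass and fog through the MC_Environment material parameter collection and tint the directional light in step.
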(event `self.ReceiveBeginPlay`
  (bind _fireflies (`self.FireFlies`))
  (`NiagaraComponent.SetVariableLinearColor` _fireflies "PaticleColor" (`self.In Value`))
  (`NiagaraComponent.SetVariableFloat` _fireflies "WindSpeedScale" 1000.0))

(fn `UserConstructionScript`)