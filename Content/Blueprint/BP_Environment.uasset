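; Environment actor that configures a firefly particle effect and holds logic for shifting scene colors.
; BeginPlay sets the fireflies' scale color and spawn rate.
; A self-restarting timeline would blend grass and fog colors in the MC_Environment parameter collection along with the directional light's color.
; Nothing starts that timeline, so the color cycle never runs.
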(event `self.ReceiveBeginPlay`
  (bind _fireflies (`self.FireFlies`))
  (`NiagaraComponent.SetVariableLinearColor` _fireflies "ScaleColor" (`self.In Value`))
  (`NiagaraComponent.SetVariableFloat` _fireflies "SpawnRate" 10000.0))

(fn `UserConstructionScript`)