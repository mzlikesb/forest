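; BP_Box is a networked interactable box that one actor at a time can focus, shown through changes to its cube's scale.
; On authority, Focus claims a free box and calls SetOwner, presumably enabling the owning client's Interact-to-InteractServer call, while Leave clears OwnerActor only for that owner.
; Multicast events drive the visuals: focus plays a scale timeline, interact flattens the cube, and leave restores its scale.
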(event `LeaveMulticast`
  (`KismetSystemLibrary.PrintString` "leave")
  (`TimelineComponent.Stop` (`self.Timeline`))
  (`SceneComponent.SetRelativeScale3D` (`self.Cube`) (`KismetMathLibrary.Vector_One`)))

(event `/Game/Blueprint/BI_Intreactable.Leave`
  (params (Owner :type "Actor Object Reference"))
  (bind _owneractor (`self.OwnerActor`))
  (`/Engine/EditorBlueprintResources/ActorMacros.Switch Has Authority`
    (:`Authority`
      (`/Engine/EditorBlueprintResources/StandardMacros.IsValid` _owneractor
        (:`Is Valid`
          (if (== Owner _owneractor)
            (set `self.OwnerActor` null)
            (`self.LeaveMulticast`)))))))

(event `InteractServer`
  (`self.InteractMulticast`))

(event `/Game/Blueprint/BI_Intreactable.Interact`
  (`self.InteractServer`))

(event `InteractMulticast`
  (`TimelineComponent.Stop` (`self.Timeline`))
  (`SceneComponent.SetRelativeScale3D` (`self.Cube`) (1.0 1.0 0.2)))

(event `/Game/Blueprint/BI_Intreactable.Focus`
  (params (Owner :type "Actor Object Reference"))
  (`/Engine/EditorBlueprintResources/ActorMacros.Switch Has Authority`
    (:`Authority`
      (`/Engine/EditorBlueprintResources/StandardMacros.IsValid` (`self.OwnerActor`)
        (:`Is Not Valid`
          (bind _output_get (set `self.OwnerActor` Owner))
          (`self.SetOwner` _output_get)
          (`self.FocusMulticast`))))))

(event `FocusMulticast`
  (bind (_direction _size) (`Timeline|Timeline` :!via `PlayFromStart`)
    (:`Update`
      (`SceneComponent.SetRelativeScale3D` (`self.Cube`) (* _size (`KismetMathLibrary.Vector_One`))))))

(fn `IsInteractable`
  (returns (isInteractable :type Boolean))
  (return (== (`self.OwnerActor`) null)))

(fn `UserConstructionScript`)