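; BP_EntryPC is the player controller for the entry screen, handling its main menu and loading UI.
; On BeginPlay it creates and shows the WB_Entry widget, sets Game and UI input mode and shows the mouse cursor.
; GetWidet lazily creates and caches the entry widget, while ShowLoading clears all widgets and displays a cached or newly created WB_Loading screen.
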(event `self.ReceiveBeginPlay`
  (`self.GetWidet`)
  (`WidgetBlueprintLibrary.SetInputMode_GameAndUIEx` self null)
  (set `self.bShowMouseCursor` true))

(fn `GetWidet`
  (returns (Output_Get :type "/Game/Blueprints/WB_Entry Object Reference"))
  (`/Engine/EditorBlueprintResources/StandardMacros.IsValid` (`self.MainWidget`)
    (:`Is Valid`
      (return (`self.MainWidget`)))
    (:`Is Not Valid`
      (bind _returnvalue (`|CreateWidget` "/Game/Blueprints/WB_Entry.WB_Entry_C"))
      (bind _output_get (set `self.MainWidget` _returnvalue))
      (`UserWidget.AddToViewport` _output_get 0)
      (return _output_get))))

(fn `ShowLoading`
  (`WidgetLayoutLibrary.RemoveAllWidgets`)
  (`/Engine/EditorBlueprintResources/StandardMacros.IsValid` (`self.LoadingWidget`)
    (:`Is Valid`
      (`UserWidget.AddToViewport` (`self.LoadingWidget`) 0))
    (:`Is Not Valid`
      (bind _returnvalue (`|CreateWidget` "/Game/Blueprints/WB_Loading.WB_Loading_C"))
      (set `self.LoadingWidget` _returnvalue)
      (`UserWidget.AddToViewport` (`self.LoadingWidget`) 0))))

(fn `UserConstructionScript`)