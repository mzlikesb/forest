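; BP_NPC is an NPC actor that maintains a smoothed look-at point for nearby player or other BP_Character pawns.
; Each Tick, FindTarget takes the first BP_Character from a sphere overlap within InteractionRange.
; LookTarget returns a point above that character, or a default point along the mesh's right vector when none is found.
; The Target vector lerps toward that point at a frame-time-scaled rate.
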(event `self.ReceiveActorBeginOverlap`
  (params (OtherActor :type "Actor Object Reference")))

(event `self.ReceiveTick`
  (params (DeltaSeconds :type "Float (single-precision)"))
  (bind _target (`self.FindTarget`))
  (bind _targetlocation (`self.LookTarget` _target))
  (bind _output_get (set `self.PrevTarget` (`self.Target`)))
  (set `self.Target` (`KismetMathLibrary.VLerp` _output_get _targetlocation (* DeltaSeconds 5.0))))

(fn `FindTarget`
  (returns (Target :type "Actor Object Reference"))
  (bind (_outactors _returnvalue) (`KismetSystemLibrary.SphereOverlapActors` (`self.K2_GetActorLocation`) (`self.InteractionRange`) (`|MakeArray` "ObjectTypeQuery3" :!type "EObjectTypeQuery Enum") "/Game/Frameworks/BP_Character.BP_Character_C"))
  (if _returnvalue
    (return (`|GetArrayItem` _outactors))
    (else
      (return null))))

(fn `LookTarget`
  (params (Target :type "Actor Object Reference"))
  (returns (TargetLocation :type "Vector Structure"))
  (bind _mesh (`self.Mesh`))
  (`/Engine/EditorBlueprintResources/StandardMacros.IsValid` Target
    (:`Is Valid`
      (return (+ (`self.K2_GetActorLocation` Target) (0.0 0.0 60.0))))
    (:`Is Not Valid`
      (return (+ (`SceneComponent.K2_GetComponentLocation` _mesh) (0.0 0.0 160.0) (* (`SceneComponent.GetRightVector` _mesh) (`self.InteractionRange`)))))))

(fn `UserConstructionScript`)