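; Player controller that connects a chat widget to the player character's voice recording and to NPC messages.
; On begin play it creates the WB_Chat widget for the local player and enables game-and-UI input with a visible cursor.
; Widget record events start and finish recording on the character, while received Whisper text from the character and the first found NPC is forwarded to the chat.
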(event `self.ReceiveBeginPlay`
  (bind _chatwidet (`self.ChatWidet`))
  (`|ExecutionSequence`
    (:`then_0`
      (`self.GetWidget`)
      (`WidgetBlueprintLibrary.SetInputMode_GameAndUIEx` self null)
      (set `self.bShowMouseCursor` true))
    (:`then_1`
      (bind _asbp_character (cast `/Game/Frameworks/BP_Character` (`GameplayStatics.GetPlayerPawn` 0)))
      (add `/Game/Blueprints/WB_Chat.OnStartRecord` _chatwidet (delegate `OnStartRecord`))
      (add `/Game/Blueprints/WB_Chat.OnFinishRecord` _chatwidet (delegate `OnFinishRecord`))
      (add `/Game/Frameworks/BP_Character.OnReceiveMessage` _asbp_character (delegate `ReceiveWhisperText`)))
    (:`then_2`
      (bind _returnvalue (`GameplayStatics.GetActorOfClass` "/Game/Blueprints/BP_NPC.BP_NPC_C"))
      (add `/Game/Blueprints/BP_NPC.OnReceiveMessage` _returnvalue (delegate `OnReceiveNPCMessage`)))))

(event `OnFinishRecord`
  (`/Game/Frameworks/BP_Character.FinishRecord` (stale `self.ReceiveBeginPlay` _asbp_character)))

(event `OnStartRecord`
  (`/Game/Frameworks/BP_Character.StartRecord` (stale `self.ReceiveBeginPlay` _asbp_character)))

(event `ReceiveWhisperText`
  (params (Text :type String) (bIsUser :type Boolean))
  (`/Game/Blueprints/WB_Chat.ReceiveWhisperText` (`self.ChatWidet`) Text bIsUser))

(event `OnReceiveNPCMessage`
  (params (Text :type String) (bIsUser :type Boolean))
  (`/Game/Blueprints/WB_Chat.ReceiveWhisperText` (`self.ChatWidet`) Text bIsUser))

(fn `GetWidget`
  (returns (Output_Get :type "/Game/Blueprints/WB_Chat Object Reference"))
  (if (`self.IsLocalController`)
    (`/Engine/EditorBlueprintResources/StandardMacros.IsValid` (`self.ChatWidet`)
      (:`Is Valid`
        (return (`self.ChatWidet`)))
      (:`Is Not Valid`
        (bind _returnvalue (`|CreateWidget` "/Game/Blueprints/WB_Chat.WB_Chat_C"))
        (bind _output_get (set `self.ChatWidet` _returnvalue))
        (`UserWidget.AddToViewport` _output_get 0)
        (return _output_get)))))

(fn `UserConstructionScript`)