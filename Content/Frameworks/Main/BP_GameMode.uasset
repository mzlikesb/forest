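; Game mode that spawns players into a multiplayer session and keeps a shared roster of their data.
; PostLogin spawns a BP_Character at a PlayerStart, possesses it, registers the controller and initializes its player data.
; UpdatePlayerData rebuilds the data list from registered controllers, applies each player's Type to their character, then tells every controller to refresh.
; Logout removes the controller and its data entry by index without triggering a refresh.
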(event `self.K2_PostLogin`
  (params (NewPlayer :type "PlayerController Object Reference"))
  (bind _asbp_player_controller (cast `/Game/Frameworks/Main/BP_PlayerController` NewPlayer))
  (bind _returnvalue (`GameplayStatics.GetActorOfClass` "/Script/Engine.PlayerStart"))
  (bind _returnvalue_2 (`|SpawnActorFromClass` "/Game/Frameworks/BP_Character.BP_Character_C" (`self.GetTransform` _returnvalue) "Undefined" "MultiplyWithRoot" null null))
  (`Controller.Possess` _asbp_player_controller _returnvalue_2)
  (`KismetArrayLibrary.Array_Add` (`self.Players`) _asbp_player_controller)
  (`/Game/Frameworks/Main/BP_PlayerController.InitPlayerData` _asbp_player_controller))

(event `UpdatePlayerData`
  (`KismetArrayLibrary.Array_Clear` (`self.AllPlayerData`))
  (for _array_element (`self.Players`)
    (bind _playerdata (`/Game/Frameworks/Main/BP_PlayerController.PlayerData` _array_element))
    (`KismetArrayLibrary.Array_Add` (`self.AllPlayerData`) _playerdata)
    (bind _asbp_character (cast `/Game/Frameworks/BP_Character` (`Controller.K2_GetPawn` _array_element)))
    (`/Game/Frameworks/BP_Character.SetType` _asbp_character (`.Type` (break `PlayerData` _playerdata))))
  (for _array_element_2 (`self.Players`)
    (`/Game/Frameworks/Main/BP_PlayerController.UpdateAllPlayerData` :`self` _array_element_2)))

(event `self.K2_OnLogout`
  (params (ExitingController :type "Controller Object Reference"))
  (bind _asbp_player_controller (cast `/Game/Frameworks/Main/BP_PlayerController` ExitingController))
  (bind _returnvalue (`KismetArrayLibrary.Array_Find` (`self.Players`) _asbp_player_controller))
  (`KismetArrayLibrary.Array_Remove` (`self.AllPlayerData`) _returnvalue)
  (`KismetArrayLibrary.Array_Remove` (`self.Players`) _returnvalue))

(fn `UserConstructionScript`)