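; Player controller that handles player data and chat, showing the mouse cursor with game-and-UI input.
; InitPlayerData passes PlayerData from BP_GameInstance to SendPlayerData, which stores it and tells BP_GameMode to update player data.
; SendChat relays a message to every BP_PlayerController, each forwarding it to its lazily created WB_Chat widget.
; UpdateAllPlayerData is an empty stub.
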(event `self.ReceiveBeginPlay`
  (`self.GetWidet`)
  (`WidgetBlueprintLibrary.SetInputMode_GameAndUIEx` self null)
  (set `self.bShowMouseCursor` true))

(event `InitPlayerData`
  (bind _asbp_game_instance (cast `/Game/Frameworks/BP_GameInstance` (`GameplayStatics.GetGameInstance`)))
  (`self.SendPlayerData` (`/Game/Frameworks/BP_GameInstance.PlayerData` _asbp_game_instance)))

(event `SendPlayerData`
  (params (PlayerData :type "PlayerData Structure"))
  (set `self.PlayerData` PlayerData)
  (bind _asbp_game_mode (cast `/Game/Frameworks/Main/BP_GameMode` (`GameplayStatics.GetGameMode`)))
  (`/Game/Frameworks/Main/BP_GameMode.UpdatePlayerData` _asbp_game_mode))

(event `SendChat`
  (params (Chat :type Text))
  (bind _outactors (`GameplayStatics.GetAllActorsOfClass` "BP_PlayerController_C"))
  (for _array_element _outactors
    (`self.ReceiveChat` _array_element Chat)))

(event `ReceiveChat`
  (params (Chat :type Text))
  (bind _output_get (`self.GetWidet`))
  (`/Game/Blueprint/WB_Chat.ReceiveChat` _output_get Chat))

(event `UpdateAllPlayerData`
  (params (AllPlayerData :type "Array of PlayerData Structure")))

(fn `GetWidet`
  (returns (Output_Get :type "/Game/Blueprint/WB_Chat Object Reference"))
  (`/Engine/EditorBlueprintResources/StandardMacros.IsValid` (`self.ChatWidet`)
    (:`Is Valid`
      (return (`self.ChatWidet`)))
    (:`Is Not Valid`
      (bind _returnvalue (`|CreateWidget` "/Game/Blueprint/WB_Chat.WB_Chat_C"))
      (bind _output_get (set `self.ChatWidet` _returnvalue))
      (`UserWidget.AddToViewport` _output_get 0)
      (return _output_get))))

(fn `UserConstructionScript`)